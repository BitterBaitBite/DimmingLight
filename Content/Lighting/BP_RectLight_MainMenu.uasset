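; Rect light for the main menu that flickers at random.
; BeginPlay caches the light's starting intensity as the maximum.
; Tick runs through a short Delay, which throttles updates, then eases the current intensity partway toward a random fraction of that maximum, clamped to a minimum floor.
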(event EventTick
  (params (DeltaSeconds :type Float%20%28single-precision%29))
  (bind _rectlightcomponent (Variables|Default|GetRectLightComponent))
  (Utilities|FlowControl|Delay 0.2)
  (Rendering|Components|Light|SetIntensity _rectlightcomponent (Math|Float|Lerp (Variables|/Script/Engine.LightComponentBase|GetIntensity _rectlightcomponent) (* (Variables|Default|GetMaxIntensity) (Math|Float|Clamp(Float) (Math|Random|RandomFloat) (Variables|Default|GetMinIntensity))) 0.3)))

(event EventBeginPlay
  (Variables|Default|SetMaxIntensity (Variables|/Script/Engine.LightComponentBase|GetIntensity (Variables|Default|GetRectLightComponent))))

(fn ConstructionScript)