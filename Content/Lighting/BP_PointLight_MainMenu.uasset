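; BP_PointLight_MainMenu is a point light, named for the main menu, that flickers randomly.
; BeginPlay stores the component's starting intensity as the maximum.
; A Delay on Tick throttles updates to roughly five per second.
; Each update lerps the current intensity partway toward a random fraction of that maximum, floored by MinIntensity, to soften the flicker.
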(event EventTick
  (params (DeltaSeconds :type Float%20%28single-precision%29))
  (bind _pointlightcomponent (Variables|Default|GetPointLightComponent))
  (Utilities|FlowControl|Delay 0.2)
  (Rendering|Components|Light|SetIntensity _pointlightcomponent (Math|Float|Lerp (Variables|/Script/Engine.LightComponentBase|GetIntensity _pointlightcomponent) (* (Variables|Default|GetMaxIntensity) (Math|Float|Clamp(Float) (Math|Random|RandomFloat) (Variables|Default|GetMinIntensity))) 0.3)))

(event EventBeginPlay
  (Variables|Default|SetMaxIntensity (Variables|/Script/Engine.LightComponentBase|GetIntensity (Variables|Default|GetPointLightComponent))))

(fn ConstructionScript)